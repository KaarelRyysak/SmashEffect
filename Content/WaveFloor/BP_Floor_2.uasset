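; BP_Floor_2 is a floor Blueprint that records impacts for up to four waves, likely rendered by a material.
; A custom hit event writes each location into the next MPC_CollsionDetails2 slot and stores its game time.
; A counter picks the slot and resets to 1 after the fourth, so the first slot is never reused.
; Tick is empty, and the older single-wave timing logic driving TimeFromImpact is disconnected.
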(event Custom|CustomEvent
  (params (MyComp :type Primitive%20Component%20Object%20Reference) (Other :type Actor%20Object%20Reference) (OtherComp :type Primitive%20Component%20Object%20Reference) (bSelfMoved :type Boolean) (HitLocation :type Vector) (HitNormal :type Vector) (NormalImpulse :type Vector) (Hit :type Hit%20Result%20Structure%20%28by%20ref%29))
  (bind _returnvalue (Actor|GetGameTimeSinceCreation))
  (bind _returnvalue_2 (Math|Conversions|ToLinearColor(Vector) HitLocation))
  (Variables|Default|SetHit true)
  (if true
    (if (== (Variables|Default|GetWavenumber) 0)
      (Rendering|Material|SetVectorParameterValue "/Game/Materials/MPC_CollsionDetails2.MPC_CollsionDetails2" "HitLocation1" _returnvalue_2 :!class /Script/Engine.KismetMaterialLibrary)
      (Variables|Default|SetWave1ImpactStart _returnvalue)
      (Variables|Default|SetWavenumber (+ (Variables|Default|GetWavenumber) 1) :!label _label)
      (elif (== (Variables|Default|GetWavenumber) 1)
        (Rendering|Material|SetVectorParameterValue "/Game/Materials/MPC_CollsionDetails2.MPC_CollsionDetails2" "HitLocation2" _returnvalue_2 :!class /Script/Engine.KismetMaterialLibrary)
        (Variables|Default|SetWave2ImpactStart _returnvalue)
        (goto _label)
        (elif (== (Variables|Default|GetWavenumber) 2)
          (Rendering|Material|SetVectorParameterValue "/Game/Materials/MPC_CollsionDetails2.MPC_CollsionDetails2" "HitLocation3" _returnvalue_2 :!class /Script/Engine.KismetMaterialLibrary)
          (Variables|Default|SetWave3ImpactStart _returnvalue)
          (goto _label)
          (elif (== (Variables|Default|GetWavenumber) 3)
            (Rendering|Material|SetVectorParameterValue "/Game/Materials/MPC_CollsionDetails2.MPC_CollsionDetails2" "HitLocation4" _returnvalue_2 :!class /Script/Engine.KismetMaterialLibrary)
            (Variables|Default|SetWave4ImpactStart _returnvalue)
            (Variables|Default|SetWavenumber 1)))))))

(event EventTick
  (params (DeltaSeconds :type Float%20%28single-precision%29)))

(fn ConstructionScript)