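; Floor actor that reacts to projectile hits with a wave driven through the MPC_CollsionDetails material parameter collection and with impact particles.
; Hit writes the impact location to the collection and sets the Wave flag.
; While flagged, Tick writes TimeFromImpact from time since LastWaveEnd, clearing the flag once the duration elapses.
; A branching macro selects the emitter spawned just above the impact by projectile class.
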(event Collision|EventHit
  (params (MyComp :type Primitive%20Component%20Object%20Reference) (Other :type Actor%20Object%20Reference) (OtherComp :type Primitive%20Component%20Object%20Reference) (bSelfMoved :type Boolean) (HitLocation :type Vector :default "0, 0, 0") (HitNormal :type Vector :default "0, 0, 0") (NormalImpulse :type Vector :default "0, 0, 0") (Hit :type Hit%20Result%20Structure%20%28by%20ref%29))
  (bind _returnvalue (Utilities|GetClass Other))
  (bind _returnvalue_2 (+ HitLocation "0, 0,20.000000"))
  (Variables|Default|SetHit true)
  (if (Variables|Default|GetHit)
    (Variables|Default|SetHit false)
    (Rendering|Material|SetVectorParameterValue "/Game/Materials/World/MPC_CollsionDetails.MPC_CollsionDetails" "HitLocation" (Math|Conversions|ToLinearColor(Vector) HitLocation) :!class /Script/Engine.KismetMaterialLibrary)
    (Variables|Default|SetWave true)
    (Utilities|NewMacro1 (== _returnvalue "/Game/FirstPersonBP/Blueprints/FirstPersonProjectileFire.FirstPersonProjectileFire_C") (== _returnvalue "/Game/FirstPersonBP/Blueprints/FirstPersonProjectileIce.FirstPersonProjectileIce_C") (== _returnvalue "/Game/FirstPersonBP/Blueprints/FirstPersonProjectileRock.FirstPersonProjectileRock_C") (== _returnvalue "/Game/FirstPersonBP/Blueprints/FirstPersonProjectileIron.FirstPersonProjectileIron_C") (== _returnvalue "/Game/FirstPersonBP/Blueprints/FirstPersonProjectileTest.FirstPersonProjectileTest_C")
      (:then
        (Effects|SpawnEmitteratLocation "/Game/FirstPersonBP/ParticleEffects/PS_Fire_Burst.PS_Fire_Burst" _returnvalue_2))
      (:then2
        (Effects|SpawnEmitteratLocation "/Game/FirstPersonBP/ParticleEffects/FlyingRocks.FlyingRocks" _returnvalue_2))
      (:then3
        (Effects|SpawnEmitteratLocation "/Game/FirstPersonBP/ParticleEffects/SparkPartSys.SparkPartSys" _returnvalue_2 "90.000000, 0, 0"))
      (:then4
        (Effects|SpawnEmitteratLocation "/Game/FirstPersonBP/ParticleEffects/Vector_Tornado.Vector_Tornado" _returnvalue_2)))))

(event Collision|EventActorBeginOverlap
  (params (OtherActor :type Actor%20Object%20Reference)))

(event EventBeginPlay)

(event EventTick
  (params (DeltaSeconds :type Float%20%28single-precision%29))
  (bind _returnvalue (Actor|GetGameTimeSinceCreation))
  (bind _returnvalue_2 (/ _returnvalue 0.1))
  (if (Variables|Default|GetWave)
    (Rendering|Material|GetVectorParameterValue "/Game/Materials/World/MPC_CollsionDetails.MPC_CollsionDetails" "HitLocation" :!class /Script/Engine.KismetMaterialLibrary)
    ;[1 1 1] If it's bigger than one, restart the wave and try again
    (if (>= (/ (- _returnvalue_2 (Variables|Default|GetLastWaveEnd)) 2e+01) 1.0)
      (Variables|Default|SetWave false)
      (Variables|Default|SetLastWaveEnd _returnvalue_2))
    ;[1 1 1] This has to be set from 0 to 1. 0=wave start, 1=wave end
    (Rendering|Material|SetScalarParameterValue "/Game/Materials/World/MPC_CollsionDetails.MPC_CollsionDetails" "TimeFromImpact" (/ (- _returnvalue_2 (Variables|Default|GetLastWaveEnd)) 2e+01) :!class /Script/Engine.KismetMaterialLibrary)
    (if true
      _)))

(fn ConstructionScript)